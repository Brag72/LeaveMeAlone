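; BP_Gate is a double gate that swings open when a player carrying a key walks into its trigger.
; The Box overlap casts to CH_Player and, if EquippedKey is above zero, decrements it and plays the GateSwitcher timeline.
; The timeline alpha lerps the relative yaw of the left and right gate roots in opposite directions.
; No open-state check guards this, so every qualifying overlap consumes a key.
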(event OnComponentBeginOverlap(Box)
  (params (OverlappedComponent :type Primitive%20Component%20Object%20Reference) (OtherActor :type Actor%20Object%20Reference) (OtherComp :type Primitive%20Component%20Object%20Reference) (OtherBodyIndex :type Integer) (bFromSweep :type Boolean) (SweepResult :type Hit%20Result%20Structure%20%28by%20ref%29))
  (bind _asch_player (Utilities|Casting|CastToCH_Player OtherActor))
  (if (> (Variables|/Script/LeaveMeAlone.LMADefaultCharacter|GetEquippedKey _asch_player) 0)
    (Math|Integer|DecrementInt (Variables|/Script/LeaveMeAlone.LMADefaultCharacter|GetEquippedKey _asch_player)
      (:%20%20
        (bind _gateswitcheralpha (Timeline|GateSwitcher Play)
          (:Update
            (Transformation|SetRelativeRotation (Variables|Default|GetLeftGateRoot) (Math|Rotator|Lerp(Rotator) "0, 0, 0" "0.000000,-50.000000,0.000000" _gateswitcheralpha) false false)
            (Transformation|SetRelativeRotation (Variables|Default|GetRightGateRoot) (Math|Rotator|Lerp(Rotator) "0, 0, 0" "0.000000,50.000000,0.000000" _gateswitcheralpha) false false)))))))

(event EventBeginPlay)

(event Collision|EventActorBeginOverlap
  (params (OtherActor :type Actor%20Object%20Reference)))

(event EventTick
  (params (DeltaSeconds :type Float%20%28single-precision%29)))

(fn ConstructionScript)