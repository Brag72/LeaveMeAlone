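; Base grenade actor that launches itself forward, explodes after a randomized fuse and damages nearby enemies.
; Shortly after BeginPlay, its Sphere gets a forward velocity impulse scaled by ScaleImpulse.
; On detonation it calls Explosive, then sphere-overlaps pawns and passes damage straight to each CH_Enemy's health widget rather than through engine damage.
; It finally spawns a radius-scaled explosion effect and destroys itself.
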(event EventBeginPlay
  (bind _sphere (Variables|Default|GetSphere))
  (bind _timetoexplode (Variables|Default|GetTimeToExplode))
  (Utilities|FlowControl|Delay 0.1)
  (Physics|AddImpulse _sphere (* (Math|Vector|GetForwardVector _sphere) 1.8e+03 (Math|Float|MapRangeClamped (Variables|Default|GetScaleImpulse) 0.0 1.5e+03 0.0 1.0)) "None" true)
  (Utilities|FlowControl|Delay (Math|Random|RandomFloatinRange (- _timetoexplode 1.0) (+ _timetoexplode 1.0)))
  (Class|LMAGrenadeBase|Explosive)
  (bind _outactors (Collision|SphereOverlapActors (Transformation|GetActorLocation) (Variables|Default|GetExplosiveRadius) (Utilities|Array|MakeArray "ObjectTypeQuery3") 0))
  (for _array_element _outactors
    (bind _asch_enemy (Utilities|Casting|CastToCH_Enemy _array_element))
    (bind _aswbp_enemy_health (Utilities|Casting|CastToWBP_EnemyHealth (UserInterface|GetWidget (Variables|/Game/LeaveMeAlone/Core/Character/CH_Enemy.CH_Enemy_C|GetWidget _asch_enemy))))
    (Default|UpdateHealth _aswbp_enemy_health (Variables|Default|GetDamageExplosive) _asch_enemy))
  (Niagara|SpawnSystematLocation "/Game/StarterContent/Particles/P_Explosion_Converted.P_Explosion_Converted" (Transformation|GetActorLocation) "0, 0, 0" (Math|Conversions|ToVector(Float) (/ (Variables|Default|GetExplosiveRadius) 1e+02)))
  (Actor|DestroyActor))

(event Collision|EventActorBeginOverlap
  (params (OtherActor :type Actor%20Object%20Reference)))

(event EventTick
  (params (DeltaSeconds :type Float%20%28single-precision%29)))

(fn ConstructionScript)